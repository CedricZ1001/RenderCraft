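; BP_Render is the Nicole character's render Blueprint, driving SDF face shading from the directional light.
; Its construction script makes the outline mesh follow Ni2's pose, creates a dynamic face material and starts a 0.01-second looping timer.
; Each timer tick compares the light's forward vector with the head socket's location using cross and dot products, then writes the result to SDF_Offset.
; The first DirectionalLight found becomes the target when none is set.
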(event `Begin Update`
  (`KismetSystemLibrary.K2_SetTimerDelegate` (delegate `Update SDF Loction`) 0.01 true)
  (bind _returnvalue (`KismetMaterialLibrary.CreateDynamicMaterialInstance` (`self.FaceMaterialInst`)))
  (bind _output_get (set `self.DynamicFaceMaterial` _returnvalue))
  (`PrimitiveComponent.SetMaterial` (`self.ni2`) (`KismetArrayLibrary.Array_Find` (`MeshComponent.GetMaterials` (`self.ni2`)) (`self.FaceMaterialInst`)) _output_get))

(event `Update SDF Loction`
  (bind _returnvalue (`SceneComponent.GetSocketLocation` (`self.ni2`) (`self.HeadBoneName`)))
  (bind _returnvalue_2 (`KismetMathLibrary.GetForwardVector` (`self.K2_GetActorRotation` (`self.LightTarget`))))
  (bind (_returnvalue_x _returnvalue_y _returnvalue_z) (`KismetMathLibrary.BreakVector` (`KismetMathLibrary.Cross_VectorVector` _returnvalue_2 _returnvalue)))
  (bind _returnvalue_3 (`KismetMathLibrary.Dot_VectorVector` _returnvalue_2 _returnvalue))
  (`self.LightTarget`
    (:`then`
      _)
    (:`else`
      (bind _outactors (`GameplayStatics.GetAllActorsOfClass` "/Script/Engine.DirectionalLight"))
      (bind _output (`|GetArrayItem` _outactors))
      (`/Engine/EditorBlueprintResources/StandardMacros.IsValid` _output
        (:`Is Valid`
          (set `self.LightTarget` _output)))))
  (if (<= _returnvalue_z 0.0)
    (if (<= _returnvalue_3 0.0)
      (set `self.SDF_Location` (/ (- -2.0 _returnvalue_3) -2.0))
      (else
        (set `self.SDF_Location` (/ (+ (- 1.0 _returnvalue_3) 1.0) -2.0))))
    (else
      (set `self.SDF_Location` (/ _returnvalue_3 2.0))))
  (`MaterialInstanceDynamic.SetScalarParameterValue` (`self.DynamicFaceMaterial`) "SDF_Offset" (`self.SDF_Location`)))

(fn `UserConstructionScript`
  (`SkinnedMeshComponent.SetLeaderPoseComponent` (`self.SM_NIcole_OutLine`) (`self.ni2`) false false)
  (`self.Begin Update`))